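; Endless-runner player character that constantly runs along world X, switches between five corridors and keeps a coin count.
; StrafeLeft and StrafeRight change a clamped DesiredCorridor index, which Tick follows with swept SetActorLocation steps along Y at StrafeSpeed.
; Die fires once, freezing movement and input, playing explosion effects and hiding the mesh, then restarts the level after a delay.
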(event `self.ReceiveBeginPlay`)

(event `self.ReceiveTick`
  (params (DeltaSeconds :type "Float (single-precision)"))
  (bind (_returnvalue_x _returnvalue_y) (`KismetMathLibrary.BreakVector` (`self.K2_GetActorLocation`)))
  (bind _returnvalue (- (`/Game/Blueprints/BPF_Run.Get Corridor Y` (`self.Desired Corridor`)) _returnvalue_y))
  (if (not (`self.Is Dead`))
    ;[1 1 1] Perpetual forward motion
    (`self.AddMovementInput` (1.0 0.0 0.0))
    (if (> (`KismetMathLibrary.Abs` _returnvalue) 5.0)
      (`self.K2_SetActorLocation` (+ (`self.K2_GetActorLocation`) (`KismetMathLibrary.MakeVector` 0.0 (* DeltaSeconds (`self.Strafe Speed`) (`KismetMathLibrary.SignOfFloat` _returnvalue)))) true))))

(event `Die`
  (bind _returnvalue (`self.K2_GetActorLocation`))
  (if (not (`self.Is Dead`))
    (set `self.Is Dead` true)
    (`MovementComponent.StopMovementImmediately` (`self.CharacterMovement`))
    (`self.DisableInput` null)
    (`GameplayStatics.SpawnEmitterAtLocation` "/Game/StarterContent/Particles/P_Explosion.P_Explosion" _returnvalue)
    (`GameplayStatics.PlaySoundAtLocation` "/Game/StarterContent/Audio/Explosion_Cue.Explosion_Cue" _returnvalue (struct) 1.0 1.0 0.0 null null null null)
    (`SceneComponent.SetVisibility` (`self.Mesh`) false false)
    (`KismetSystemLibrary.Delay` 3.0)
    (`KismetSystemLibrary.ExecuteConsoleCommand` "RestartLevel" null)))

(fn `Add Coin`
  (`/Engine/EditorBlueprintResources/StandardMacros.IncrementInt` (`self.Coins`)))

(fn `Strafe Left`
  (bind _desired_corridor (`self.Desired Corridor`))
  (if (!= _desired_corridor 0)
    (`/Engine/EditorBlueprintResources/StandardMacros.DecrementInt` _desired_corridor)))

(fn `Strafe Right`
  (bind _result (`/Engine/EditorBlueprintResources/StandardMacros.IncrementInt` (`self.Desired Corridor`))
    (:`  `
      (if (== _result 5)
        (set `self.Desired Corridor` 4)))))

(fn `UserConstructionScript`)