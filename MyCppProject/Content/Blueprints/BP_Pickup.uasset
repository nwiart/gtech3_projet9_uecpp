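; BP_Pickup is a base collectible actor that reacts when the player's BP_RunCharacter touches it.
; Its static mesh's begin-overlap checks for player character 0, casts it to BP_RunCharacter and passes it to OnHit, an empty hook for the pickup's effect.
; It then plays PickupSound at its location, if one is set, and destroys itself.
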(event `self.StaticMesh.OnComponentBeginOverlap`
  (params (OverlappedComponent :type "PrimitiveComponent Object Reference") (OtherActor :type "Actor Object Reference") (OtherComp :type "PrimitiveComponent Object Reference") (OtherBodyIndex :type Integer) (bFromSweep :type Boolean) (SweepResult :type "HitResult Structure (by ref)"))
  (bind _returnvalue (`GameplayStatics.GetPlayerCharacter` 0))
  (if (== OtherActor _returnvalue)
    (bind _asbp_run_character (cast `/Game/Blueprints/Characters/BP_RunCharacter` _returnvalue))
    (`self.OnHit` _asbp_run_character)
    (`/Engine/EditorBlueprintResources/StandardMacros.IsValid` (`self.Pickup Sound`)
      (:`Is Valid`
        (`GameplayStatics.PlaySoundAtLocation` (`self.Pickup Sound`) (`self.K2_GetActorLocation`) (struct) 1.0 1.0 0.0 null null null null))
      (:`Is Not Valid`
        _))
    (`self.K2_DestroyActor`)))

(fn `OnHit`
  (params (`Run Character` :type "/Game/Blueprints/Characters/BP_RunCharacter Object Reference")))

(fn `UserConstructionScript`)