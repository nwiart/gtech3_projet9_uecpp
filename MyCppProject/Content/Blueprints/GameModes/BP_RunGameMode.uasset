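; BP_RunGameMode is the game mode for an endless runner, creating the run HUD widget and generating the floor.
; At BeginPlay it spawns an initial chain of floor tiles, each placed at the attach transform of the previous one.
; Each tile's exit event spawns a new tile at the front and destroys the exited tile after a short delay, keeping the track rolling.
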(event `self.ReceiveBeginPlay`
  (bind _returnvalue (`|CreateWidget` "/Game/Blueprints/UI/WB_Run.WB_Run_C"))
  (`UserWidget.AddToViewport` _returnvalue 0)
  (for _ (range (+ (+ (`self.Num Initial Tiles`) 1) 1))
    (`self.Spawn Floor Tile`)))

(event `On Tile Exit`
  (params (Tile :type "/Game/Blueprints/BP_FloorTile Object Reference"))
  (`self.Spawn Floor Tile`)
  (`KismetSystemLibrary.Delay` 1.0)
  (`self.K2_DestroyActor` Tile))

(fn `Spawn Floor Tile`
  (bind _returnvalue (`|SpawnActorFromClass` "/Game/Blueprints/BP_FloorTile.BP_FloorTile_C" (`self.Current Transform`) "Undefined" "MultiplyWithRoot" null null))
  (add `/Game/Blueprints/BP_FloorTile.OnTileExit` _returnvalue (`|CreateDelegate` :!event `On Tile Exit`))
  (bind _transform (`/Game/Blueprints/BP_FloorTile.GetAttachTransform` _returnvalue))
  (set `self.Current Transform` _transform))

(fn `UserConstructionScript`)