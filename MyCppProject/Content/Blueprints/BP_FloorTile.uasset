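; BP_FloorTile is a floor segment that places its own obstacle and can be chained to other pieces.
; On BeginPlay it adds a child actor of a random ObstacleTypes class, offset in Y to one of five random corridors.
; GetAttachTransform exposes the Arrow's world transform as an attach point.
; When the player character stops at or enters BoxExit, it fires the OnTileExit dispatcher with itself.
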(event `self.ReceiveBeginPlay`
  (`self.SpawnObstacle`))

(event `self.BoxExit.OnComponentBeginOverlap`
  (params (OverlappedComponent :type "PrimitiveComponent Object Reference") (OtherActor :type "Actor Object Reference") (OtherComp :type "PrimitiveComponent Object Reference") (OtherBodyIndex :type Integer) (bFromSweep :type Boolean) (SweepResult :type "HitResult Structure (by ref)"))
  (if (== OtherActor (`GameplayStatics.GetPlayerCharacter` 0))
    (`self.OnTileExit` self)))

(fn `GetAttachTransform`
  (returns (Transform :type "Transform Structure"))
  (return (`SceneComponent.K2_GetComponentToWorld` (`self.Arrow`))))

(fn `SpawnObstacle`
  (bind _returnvalue (`AddComponent|NODE_AddChildActorComponent-0` :`RelativeTransform` (`KismetMathLibrary.MakeTransform` (`KismetMathLibrary.MakeVector` 0.0 (`/Game/Blueprints/BPF_Run.Get Corridor Y` (`KismetMathLibrary.RandomInteger` 5))))))
  (`ChildActorComponent.SetChildActorClass` _returnvalue (`KismetArrayLibrary.Array_Random` (`self.Obstacle Types`))))

(fn `UserConstructionScript`)