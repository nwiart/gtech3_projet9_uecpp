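; BP_FloorTile is a corridor floor segment that carries a random obstacle and signals when the player leaves it.
; On BeginPlay it spawns a random obstacle class in one of five corridor lanes along Y and attaches it to itself with relative transforms.
; Overlap of the exit box by the player character calls OnTileExit with the tile.
; GetAttachTransform exposes the arrow's world transform as an attach point.
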(event `self.ReceiveBeginPlay`
  (`self.SpawnObstacle`))

(event `self.BoxExit.OnComponentBeginOverlap`
  (params (OverlappedComponent :type "PrimitiveComponent Object Reference") (OtherActor :type "Actor Object Reference") (OtherComp :type "PrimitiveComponent Object Reference") (OtherBodyIndex :type Integer) (bFromSweep :type Boolean) (SweepResult :type "HitResult Structure (by ref)"))
  (if (== OtherActor (`GameplayStatics.GetPlayerCharacter` 0))
    (`self.OnTileExit` self)))

(fn `GetAttachTransform`
  (returns (Transform :type "Transform Structure"))
  (return (`SceneComponent.K2_GetComponentToWorld` (`self.Arrow`))))

(fn `SpawnObstacle`
  (bind _returnvalue (`|SpawnActorFromClass` (`KismetArrayLibrary.Array_Random` (`self.Obstacle Types`)) (`KismetMathLibrary.MakeTransform` (`KismetMathLibrary.MakeVector` 0.0 (`/Game/Blueprints/BPF_Run.Get Corridor Y` (`KismetMathLibrary.RandomInteger` 5)))) "AlwaysSpawn" "MultiplyWithRoot" null null))
  (`self.K2_AttachToActor` _returnvalue self "None" "KeepRelative" "KeepRelative" "KeepRelative" true))

(fn `UserConstructionScript`)